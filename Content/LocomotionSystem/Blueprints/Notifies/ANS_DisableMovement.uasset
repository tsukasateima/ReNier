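; Anim notify state that freezes a character's movement for the duration of a notify window in an animation.
; On begin, it casts the mesh owner to Character and disables movement on its CharacterMovement component.
; On end, it sets the movement mode back to Walking, regardless of the mode that was active before.
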(fn `Received_NotifyBegin`
  (params (MeshComp :type "SkeletalMeshComponent Object Reference") (Animation :type "AnimSequenceBase Object Reference") (TotalDuration :type "Float (single-precision)") (EventReference :type "AnimNotifyEventReference Structure (by ref)"))
  (returns (ReturnValue :type Boolean))
  (bind `_as角色` (cast `Character` (`ActorComponent.GetOwner` MeshComp)))
  (`CharacterMovementComponent.DisableMovement` (`Character.CharacterMovement` `_as角色`))
  (return true))

(fn `Received_NotifyEnd`
  (params (MeshComp :type "SkeletalMeshComponent Object Reference") (Animation :type "AnimSequenceBase Object Reference") (EventReference :type "AnimNotifyEventReference Structure (by ref)"))
  (returns (ReturnValue :type Boolean))
  (bind `_as角色` (cast `Character` (`ActorComponent.GetOwner` MeshComp)))
  (`CharacterMovementComponent.SetMovementMode` (`Character.CharacterMovement` `_as角色`) "MOVE_Walking" 0)
  (return true))